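; Sky actor that keeps a panning-cloud sky dome in sync with a Sun directional light and a Moon light for day and night.
; Construction creates a dynamic sky material and seeds its colours, clouds and stars, from color curves or manual settings.
; Each tick derives sun height from Sun pitch to update directions, curve-driven colours and star blending.
; Tick also mirrors the Moon opposite the Sun's pitch, shows only one, and boosts both intensities near the horizon.
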(event EventTick
  (params (DeltaSeconds :type Float%20%28single-precision%29))
  (bind _sun (Variables|Default|GetSun))
  (bind _relativerotation (Variables|/Script/Engine.SceneComponent|GetRelativeRotation _sun))
  (CallFunction|UpdateSunDirection)
  (Transformation|SetRelativeRotation (Variables|Default|GetMoon) (Math|Rotator|MakeRotator (.roll _relativerotation) (* (.pitch _relativerotation) -1.0) (.yaw _relativerotation)) false false)
  (if (< (.pitch _relativerotation) 0.0)
    (Development|SetHiddeninGame (Variables|Default|GetSun) false false)
    (Development|SetHiddeninGame (Variables|Default|GetMoon) true false)
    (else
      (Development|SetHiddeninGame (Variables|Default|GetSun) true false)
      (Development|SetHiddeninGame (Variables|Default|GetMoon) false false)))
  (if (< (Math|Float|Absolute(Float) (.pitch _relativerotation)) 2e+01)
    (Rendering|Components|Light|SetIntensity (Variables|Default|GetSun) 5.0)
    (else
      (Rendering|Components|Light|SetIntensity (Variables|Default|GetSun) 3.5))))

(fn ConstructionScript
  (Variables|Default|SetDirectionalLight (Variables|Default|GetSun))
  (bind _returnvalue (Rendering|Material|CreateDynamicMaterialInstance (Variables|Default|GetSkySphereMesh) 0 "/Game/Blueprints/MyBP/SkySystemTexture/M_Sky_Panning_Clouds2.M_Sky_Panning_Clouds2" "None" :!class /Script/Engine.PrimitiveComponent))
  (Variables|Default|SetSky%20material _returnvalue)
  (if (Variables|Default|GetRefresh%20material) ; Updating bool in details panel causes construction script to run again
    _
    (else
      _))
  (Variables|Default|SetRefresh%20material false)
  (CallFunction|RefreshMaterial))

(fn UpdateSunDirection
  (bind _directionallight (Variables|Default|GetDirectionalLight))
  (bind _sky_material (Variables|Default|GetSky%20material))
  (bind _sky_material_2 (Variables|Default|GetSky%20material))
  (bind _relativerotation (Variables|/Script/Engine.SceneComponent|GetRelativeRotation _directionallight))
  (bind _lightcolor (Variables|/Script/Engine.LightComponentBase|GetLightColor _directionallight))
  (bind _returnvalue (Math|Conversions|ToLinearColor(Color) _lightcolor))
  (bind _returnvalue_2 (Math|Rotator|GetRotationXVector _relativerotation))
  (Utilities|FlowControl|Sequence
    (:then_0
      (Rendering|Material|SetVectorParameterValue _sky_material "Moon direction" (Math|Conversions|ToLinearColor(Vector) (* _returnvalue_2 "-1.000000,-1.000000,-1.000000")) :!class /Script/Engine.MaterialInstanceDynamic)
      (Rendering|Material|SetVectorParameterValue _sky_material "Sun color" _returnvalue :!class /Script/Engine.MaterialInstanceDynamic))
    (:then_1
      (Rendering|Material|SetVectorParameterValue _sky_material "Light direction" (Math|Conversions|ToLinearColor(Vector) _returnvalue_2) :!class /Script/Engine.MaterialInstanceDynamic)
      (Rendering|Material|SetVectorParameterValue _sky_material "Sun color" _returnvalue :!class /Script/Engine.MaterialInstanceDynamic)
      (Variables|Default|SetSun%20height (Math|Float|MapRangeUnclamped (.Pitch (Math|Rotator|BreakRotator _relativerotation)) -9e+01 9e+01 1.0 -1.0))
      (Rendering|Material|SetVectorParameterValue _sky_material_2 "Horizon color" (Class|CurveLinearColor|GetClampedLinearColorValue (Variables|Default|GetHorizon%20color%20curve) (Variables|Default|GetSun%20height)) :!class /Script/Engine.MaterialInstanceDynamic)
      (Rendering|Material|SetVectorParameterValue _sky_material_2 "Zenith color" (Class|CurveLinearColor|GetClampedLinearColorValue (Variables|Default|GetZenith%20color%20curve) (Variables|Default|GetSun%20height)) :!class /Script/Engine.MaterialInstanceDynamic)
      (Rendering|Material|SetVectorParameterValue _sky_material_2 "Cloud color" (Class|CurveLinearColor|GetClampedLinearColorValue (Variables|Default|GetCloud%20color%20curve) (Variables|Default|GetSun%20height)) :!class /Script/Engine.MaterialInstanceDynamic)
      (Rendering|Material|SetScalarParameterValue _sky_material_2 "Horizon falloff" (Math|Float|Lerp 3.0 8.0 (Math|Float|Absolute(Float) (Variables|Default|GetSun%20height))) :!class /Script/Engine.MaterialInstanceDynamic)
      (Rendering|Material|SetScalarParameterValue _sky_material_2 "Sun height" (Math|Float|SelectFloat (Math|Float|Absolute(Float) (Variables|Default|GetSun%20height)) 0.0 (< (Variables|Default|GetSun%20height) 0.0)) :!class /Script/Engine.MaterialInstanceDynamic))))

(fn RefreshMaterial
  (bind _directionallight (Variables|Default|GetDirectionalLight))
  (bind _sky_material (Variables|Default|GetSky%20material))
  (bind _sky_material_2 (Variables|Default|GetSky%20material))
  (bind _sky_material_3 (Variables|Default|GetSky%20material))
  (bind _sky_material_4 (Variables|Default|GetSky%20material))
  (bind _sky_material_5 (Variables|Default|GetSky%20material))
  (bind _relativerotation (Variables|/Script/Engine.SceneComponent|GetRelativeRotation _directionallight))
  (Utilities|IsValid (Variables|Default|GetDirectionalLight) ; Has a directional light been assigned?
    (:Is%20Valid
      (Rendering|Material|SetVectorParameterValue _sky_material_3 "Light direction" (Math|Conversions|ToLinearColor(Vector) (Math|Rotator|GetRotationXVector _relativerotation)) :!class /Script/Engine.MaterialInstanceDynamic)
      (Rendering|Material|SetVectorParameterValue _sky_material_3 "Sun color" (Math|Conversions|ToLinearColor(Color) (Variables|/Script/Engine.LightComponentBase|GetLightColor _directionallight)) :!class /Script/Engine.MaterialInstanceDynamic)
      (Variables|Default|SetSun%20height (Math|Float|MapRangeUnclamped (.Pitch (Math|Rotator|BreakRotator _relativerotation)) -9e+01 9e+01 1.0 -1.0)))
    (:Is%20Not%20Valid
      (Rendering|Material|SetVectorParameterValue _sky_material_2 "Light direction" (Math|Conversions|ToLinearColor(Vector) (Math|Rotator|GetRotationXVector (Math|Rotator|MakeRotator 0.0 (Math|Float|MapRangeUnclamped (Variables|Default|GetSun%20height) -1.0 1.0 9e+01 -9e+01) (.Yaw (Math|Rotator|BreakRotator (Transformation|GetActorRotation)))))) :!class /Script/Engine.MaterialInstanceDynamic)
      (Rendering|Material|SetVectorParameterValue _sky_material_2 "Sun color" (Math|Color|Lerp(LinearColor) "(R=1.000000,G=0.221000,B=0.040000,A=1.000000)" "(R=0.954000,G=0.901000,B=0.744120,A=1.000000)" (Math|Float|Clamp(Float) (+ (Variables|Default|GetSun%20height) 0.2))) :!class /Script/Engine.MaterialInstanceDynamic)))
  (if (Variables|Default|GetColors%20determined%20by%20sun%20position)
    (Rendering|Material|SetVectorParameterValue _sky_material_4 "Horizon color" (Class|CurveLinearColor|GetClampedLinearColorValue (Variables|Default|GetHorizon%20color%20curve) (Variables|Default|GetSun%20height)) :!class /Script/Engine.MaterialInstanceDynamic)
    (Rendering|Material|SetVectorParameterValue _sky_material_4 "Zenith color" (Class|CurveLinearColor|GetClampedLinearColorValue (Variables|Default|GetZenith%20color%20curve) (Variables|Default|GetSun%20height)) :!class /Script/Engine.MaterialInstanceDynamic)
    (Rendering|Material|SetVectorParameterValue _sky_material_4 "Cloud color" (Class|CurveLinearColor|GetClampedLinearColorValue (Variables|Default|GetCloud%20color%20curve) (Variables|Default|GetSun%20height)) :!class /Script/Engine.MaterialInstanceDynamic)
    (Rendering|Material|SetScalarParameterValue _sky_material_4 "Horizon falloff" (Math|Float|Lerp 3.0 7.0 (Math|Float|Absolute(Float) (Variables|Default|GetSun%20height))) :!class /Script/Engine.MaterialInstanceDynamic)
    (else
      (Rendering|Material|SetVectorParameterValue _sky_material "Horizon color" (Variables|Default|GetHorizon%20color) :!class /Script/Engine.MaterialInstanceDynamic)
      (Rendering|Material|SetVectorParameterValue _sky_material "Zenith color" (Variables|Default|GetZenith%20Color) :!class /Script/Engine.MaterialInstanceDynamic)
      (Rendering|Material|SetVectorParameterValue _sky_material "Overall color" (Variables|Default|GetOverall%20Color) :!class /Script/Engine.MaterialInstanceDynamic)
      (Rendering|Material|SetVectorParameterValue _sky_material "Cloud color" (Variables|Default|GetCloud%20color) :!class /Script/Engine.MaterialInstanceDynamic)
      (Rendering|Material|SetScalarParameterValue _sky_material "Horizon falloff" (Variables|Default|GetHorizon%20Falloff) :!class /Script/Engine.MaterialInstanceDynamic)))
  (Rendering|Material|SetScalarParameterValue _sky_material_5 "Cloud speed" (Variables|Default|GetCloud%20speed) :!class /Script/Engine.MaterialInstanceDynamic)
  (Rendering|Material|SetScalarParameterValue _sky_material_5 "Sun brightness" (Variables|Default|GetSun%20brightness) :!class /Script/Engine.MaterialInstanceDynamic)
  (Rendering|Material|SetScalarParameterValue _sky_material_5 "Sun height" (Math|Float|SelectFloat (Math|Float|Absolute(Float) (Variables|Default|GetSun%20height)) 0.0 (< (Variables|Default|GetSun%20height) 0.0)) :!class /Script/Engine.MaterialInstanceDynamic)
  (Rendering|Material|SetScalarParameterValue _sky_material_5 "Cloud opacity" (Variables|Default|GetCloud%20opacity) :!class /Script/Engine.MaterialInstanceDynamic)
  (Rendering|Material|SetScalarParameterValue _sky_material_5 "Stars brightness" (Variables|Default|GetStars%20brightness) :!class /Script/Engine.MaterialInstanceDynamic))