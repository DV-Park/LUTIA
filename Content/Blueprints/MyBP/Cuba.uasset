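; Cuba is an NPC actor that plays main quest dialogue through the in-game HUD when the player's quest-clear flag is set.
; GetCommu reads DialogData1 rows keyed by quest index and line number, starting only if the first row's NPC matches the actor's name prefix.
; Each line's finished-writing event chains to the next via PlayDialog.
; A missing row ends communication, unbinds the dialog and resets the flag.
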(event Custom|PlayDialog
  (bind _as_bp_third_person_character (Variables|Default|GetAs%20BP%20Third%20Person%20Character))
  (bind _index (Variables|Default|GetIndex))
  (if (Variables|/Script/LUTIA.LUTIA_PlayerState|GetIsMainQuestClear (Variables|Default|GetAs%20LUTIA%20Player%20State))
    (bind _returnvalue (Utilities|GetDataTableRow "/Game/DataBase/DialogData1.DialogData1" (Utilities|String|StringToName (Utilities|String|Append (Utilities|String|MakeLiteralString "D_MY_") (Utilities|String|ToString(Integer) (Variables|/Script/LUTIA.LUTIA_PlayerState|GetMainQuestIndex (Variables|Default|GetAs%20LUTIA%20Player%20State))) "_" (Utilities|String|ToString(Integer) (Variables|Default|GetIndex)))))
      (:then
        (if (and (== _index 0) (Utilities|Enum|Equal(Enum) (.npc _returnvalue) (.LeftS (Utilities|String|Split (Utilities|GetObjectName self) "_"))))
          (Variables|/Script/LUTIA.LUTIACharacter|SetIsCommunicating _as_bp_third_person_character true :!label _label)
          (bind _aslutiahud (Utilities|Casting|CastToLUTIAHUD (HUD|GetHUD (Game|GetPlayerController 0))))
          (Default|Write (Variables|/Game/UMG/UMG_InGame.UMG_InGame_C|GetUMG_Dialog (Variables|/Game/Blueprints/MyBP/LUTIAHUD.LUTIAHUD_C|GetUMG_InGame _aslutiahud)) (.text _returnvalue))
          (Rendering|Components|TextRender|SetText (Variables|/Game/UMG/SubUMG/UMG_Dialog.UMG_Dialog_C|GetTxt_Name (Variables|/Game/UMG/UMG_InGame.UMG_InGame_C|GetUMG_Dialog (Variables|/Game/Blueprints/MyBP/LUTIAHUD.LUTIAHUD_C|GetUMG_InGame _aslutiahud))) (.name _returnvalue))
          (Rendering|Components|TextRender|SetText (Variables|/Game/UMG/SubUMG/UMG_Dialog.UMG_Dialog_C|GetTxt_Job (Variables|/Game/UMG/UMG_InGame.UMG_InGame_C|GetUMG_Dialog (Variables|/Game/Blueprints/MyBP/LUTIAHUD.LUTIAHUD_C|GetUMG_InGame _aslutiahud))) (.job _returnvalue))
          (Math|Integer|IncrementInt (Variables|Default|GetIndex)
            (:%20%20
              (EventDispatchers|BindEventtoFinishedWriting (Variables|/Game/UMG/UMG_InGame.UMG_InGame_C|GetUMG_Dialog (Variables|/Game/Blueprints/MyBP/LUTIAHUD.LUTIAHUD_C|GetUMG_InGame _aslutiahud)) (delegate Custom|PlayDialog))))
          (elif (!= _index 0)
            (goto _label))))
      (:RowNotFound
        (Variables|/Script/LUTIA.LUTIACharacter|SetIsCommunicating _as_bp_third_person_character false)
        (bind _aslutiahud_2 (Utilities|Casting|CastToLUTIAHUD (HUD|GetHUD (Game|GetPlayerController 0))))
        (Default|UMGUnbind (Variables|/Game/Blueprints/MyBP/LUTIAHUD.LUTIAHUD_C|GetUMG_InGame _aslutiahud_2) (Variables|/Game/UMG/UMG_InGame.UMG_InGame_C|GetUMG_Dialog (Variables|/Game/Blueprints/MyBP/LUTIAHUD.LUTIAHUD_C|GetUMG_InGame _aslutiahud_2)))
        (Variables|/Script/LUTIA.LUTIA_PlayerState|SetIsMainQuestClear (Variables|Default|GetAs%20LUTIA%20Player%20State) false)
        (Utilities|Array|SetArrayElem (Variables|/Game/UMG/UMG_InGame.UMG_InGame_C|GetIsUMGVisible (Variables|/Game/Blueprints/MyBP/LUTIAHUD.LUTIAHUD_C|GetUMG_InGame _aslutiahud_2)) 4 false)))))

(event EventBeginPlay
  (bind _asbp_third_person_character (Utilities|Casting|CastToBP_ThirdPersonCharacter (Game|Player|GetPlayerPawn 0)))
  (Variables|Default|SetAs%20BP%20Third%20Person%20Character _asbp_third_person_character)
  (bind _aslutia_player_state (Utilities|Casting|CastToLUTIA_PlayerState (Game|GetPlayerState 0)))
  (Variables|Default|SetAs%20LUTIA%20Player%20State _aslutia_player_state))

(event Collision|EventActorBeginOverlap
  (params (OtherActor :type Actor%20Object%20Reference)))

(event EventGetCommu
  (bind _as_bp_third_person_character (Variables|Default|GetAs%20BP%20Third%20Person%20Character))
  (Variables|Default|SetIndex 0)
  (if (Variables|/Script/LUTIA.LUTIA_PlayerState|GetIsMainQuestClear (Variables|Default|GetAs%20LUTIA%20Player%20State))
    (bind _returnvalue (Utilities|GetDataTableRow "/Game/DataBase/DialogData1.DialogData1" (Utilities|String|StringToName (Utilities|String|Append (Utilities|String|MakeLiteralString "D_MY_") (Utilities|String|ToString(Integer) (Variables|/Script/LUTIA.LUTIA_PlayerState|GetMainQuestIndex (Variables|Default|GetAs%20LUTIA%20Player%20State))) "_" (Utilities|String|ToString(Integer) (Variables|Default|GetIndex)))))
      (:then
        (if (and (== (Variables|Default|GetIndex) 0) (Utilities|Enum|Equal(Enum) (.npc _returnvalue) (.LeftS (Utilities|String|Split (Utilities|GetObjectName self) "_"))))
          (Variables|/Script/LUTIA.LUTIACharacter|SetIsCommunicating _as_bp_third_person_character true :!label _label)
          (bind _aslutiahud (Utilities|Casting|CastToLUTIAHUD (HUD|GetHUD (Game|GetPlayerController 0))))
          (Default|Write (Variables|/Game/UMG/UMG_InGame.UMG_InGame_C|GetUMG_Dialog (Variables|/Game/Blueprints/MyBP/LUTIAHUD.LUTIAHUD_C|GetUMG_InGame _aslutiahud)) (.text _returnvalue))
          (Rendering|Components|TextRender|SetText (Variables|/Game/UMG/SubUMG/UMG_Dialog.UMG_Dialog_C|GetTxt_Name (Variables|/Game/UMG/UMG_InGame.UMG_InGame_C|GetUMG_Dialog (Variables|/Game/Blueprints/MyBP/LUTIAHUD.LUTIAHUD_C|GetUMG_InGame _aslutiahud))) (.name _returnvalue))
          (Rendering|Components|TextRender|SetText (Variables|/Game/UMG/SubUMG/UMG_Dialog.UMG_Dialog_C|GetTxt_Job (Variables|/Game/UMG/UMG_InGame.UMG_InGame_C|GetUMG_Dialog (Variables|/Game/Blueprints/MyBP/LUTIAHUD.LUTIAHUD_C|GetUMG_InGame _aslutiahud))) (.job _returnvalue))
          (Math|Integer|IncrementInt (Variables|Default|GetIndex)
            (:%20%20
              (EventDispatchers|BindEventtoFinishedWriting (Variables|/Game/UMG/UMG_InGame.UMG_InGame_C|GetUMG_Dialog (Variables|/Game/Blueprints/MyBP/LUTIAHUD.LUTIAHUD_C|GetUMG_InGame _aslutiahud)) (delegate Custom|PlayDialog))))
          (elif (!= (Variables|Default|GetIndex) 0)
            (goto _label))))
      (:RowNotFound
        (Variables|/Script/LUTIA.LUTIACharacter|SetIsCommunicating _as_bp_third_person_character false)
        (bind _aslutiahud_2 (Utilities|Casting|CastToLUTIAHUD (HUD|GetHUD (Game|GetPlayerController 0))))
        (Default|UMGUnbind (Variables|/Game/Blueprints/MyBP/LUTIAHUD.LUTIAHUD_C|GetUMG_InGame _aslutiahud_2) (Variables|/Game/UMG/UMG_InGame.UMG_InGame_C|GetUMG_Dialog (Variables|/Game/Blueprints/MyBP/LUTIAHUD.LUTIAHUD_C|GetUMG_InGame _aslutiahud_2)))
        (Variables|/Script/LUTIA.LUTIA_PlayerState|SetIsMainQuestClear (Variables|Default|GetAs%20LUTIA%20Player%20State) false)
        (Utilities|Array|SetArrayElem (Variables|/Game/UMG/UMG_InGame.UMG_InGame_C|GetIsUMGVisible (Variables|/Game/Blueprints/MyBP/LUTIAHUD.LUTIAHUD_C|GetUMG_InGame _aslutiahud_2)) 4 false)))))

(fn ConstructionScript)