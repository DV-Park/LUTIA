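; DialogTest is a test Blueprint that plays a short scripted dialog through the player's in-game HUD.
; GetCommun builds a "SOP_" row name from DialogCount, reads that DialogData row, then sends its text and speaker name to the character's dialog widget.
; It binds itself to the widget's finished-writing event to chain lines, and passes the widget to UMGUnbind once the counter exceeds its limit.
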(event Custom|GetCommun
  (if (<= (Variables|Default|GetDialogCount) 2)
    (bind _returnvalue (Utilities|GetDataTableRow "/Game/DataBase/DialogData.DialogData" (Utilities|String|StringToName (Utilities|String|Append (Utilities|String|MakeLiteralString "SOP") "_" (Utilities|String|ToString(Integer) (Variables|Default|GetDialogCount)))))
      (:then
        (bind _asbp_third_person_character (Utilities|Casting|CastToBP_ThirdPersonCharacter (Game|Player|GetPlayerPawn 0)))
        (Default|Write (Variables|/Game/UMG/UMG_InGame.UMG_InGame_C|GetUMG_Dialog (Variables|/Game/ThirdPerson/Blueprints/BP_ThirdPersonCharacter.BP_ThirdPersonCharacter_C|GetUMG_InGame _asbp_third_person_character)) (.text _returnvalue))
        (Rendering|Components|TextRender|SetText (Variables|/Game/UMG/SubUMG/UMG_Dialog.UMG_Dialog_C|GetTxt_Name (Variables|/Game/UMG/UMG_InGame.UMG_InGame_C|GetUMG_Dialog (Variables|/Game/ThirdPerson/Blueprints/BP_ThirdPersonCharacter.BP_ThirdPersonCharacter_C|GetUMG_InGame _asbp_third_person_character))) (.name _returnvalue))
        (Math|Integer|IncrementInt (Variables|Default|GetDialogCount)
          (:%20%20
            (EventDispatchers|BindEventtoFinishedWriting (Variables|/Game/UMG/UMG_InGame.UMG_InGame_C|GetUMG_Dialog (Variables|/Game/ThirdPerson/Blueprints/BP_ThirdPersonCharacter.BP_ThirdPersonCharacter_C|GetUMG_InGame _asbp_third_person_character)) (delegate Custom|GetCommun))))))
    (else
      (bind _asbp_third_person_character_2 (Utilities|Casting|CastToBP_ThirdPersonCharacter (Game|Player|GetPlayerPawn 0)))
      (Default|UMGUnbind (Variables|/Game/ThirdPerson/Blueprints/BP_ThirdPersonCharacter.BP_ThirdPersonCharacter_C|GetUMG_InGame _asbp_third_person_character_2) (Variables|/Game/UMG/UMG_InGame.UMG_InGame_C|GetUMG_Dialog (Variables|/Game/ThirdPerson/Blueprints/BP_ThirdPersonCharacter.BP_ThirdPersonCharacter_C|GetUMG_InGame _asbp_third_person_character_2))))))

(event EventBeginPlay)

(event Collision|EventActorBeginOverlap
  (params (OtherActor :type Actor%20Object%20Reference)))

(event EventTick
  (params (DeltaSeconds :type Float%20%28single-precision%29)))

(fn ConstructionScript)