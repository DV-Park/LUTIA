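; Lantern actor whose spotlight switches on late in the world's time cycle.
; BeginPlay caches the LUTIA game state, and Tick polls its WorldTime every frame, showing the spotlight only above a fixed threshold.
; When IsOn is false, the construction script destroys the flame mesh and spotlight and zeroes the lantern's emission, though Tick still references that spotlight.
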(event EventBeginPlay
  (bind _aslutiagame_state (Utilities|Casting|CastToLUTIAGameState (Game|GetGameState)))
  (Variables|Default|SetAs%20LUTIAGame%20State _aslutiagame_state))

(event EventTick
  (params (DeltaSeconds :type Float%20%28single-precision%29))
  (bind _spotlight (Variables|Default|GetSpotLight))
  (if (> (Variables|/Script/LUTIA.LUTIAGameState|GetWorldTime (Variables|Default|GetAs%20LUTIAGame%20State)) 1.1e+03)
    (Rendering|SetVisibility _spotlight true false)
    (else
      (Rendering|SetVisibility _spotlight false false))))

(fn ConstructionScript
  (if (not (Variables|Default|GetisOn))
    (Components|DestroyComponent (Variables|Default|GetSM_Lantern_Flames))
    (Components|DestroyComponent (Variables|Default|GetSpotLight))
    (Rendering|Material|SetScalarParameterValueonMaterials (Variables|Default|GetSM_Lantern_Lantern) "Emission_Strength" 0.0)))