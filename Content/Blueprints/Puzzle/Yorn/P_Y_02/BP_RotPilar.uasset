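; BP_RotPilar is a monk pillar puzzle actor that the player can rotate through an interaction choice.
; GetCommu casts the player to BP_ThirdPersonCharacter and initializes communication on its in-game UMG.
; Select1 plays a timeline that adds its Rotate value to the mesh's current relative yaw on every update, so the turn accumulates.
; Select2 instantly adds a quarter turn of yaw.
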(event EventBeginPlay)

(event Collision|EventActorBeginOverlap
  (params (OtherActor :type Actor%20Object%20Reference)))

(event EventTick
  (params (DeltaSeconds :type Float%20%28single-precision%29)))

(event EventGetCommu
  (bind _asbp_third_person_character (Utilities|Casting|CastToBP_ThirdPersonCharacter (Game|GetPlayerCharacter 0)))
  (Default|InitCommuc (Variables|/Game/ThirdPerson/Blueprints/BP_ThirdPersonCharacter.BP_ThirdPersonCharacter_C|GetUMG_InGame _asbp_third_person_character)))

(event EventSelect1
  (bind _sm_monkpilar (Variables|Default|GetSM_MonkPilar))
  (bind _returnvalue (Transformation|GetRelativeTransform _sm_monkpilar))
  (bind _rotate (Timeline|타임라인 PlayFromStart)
    (:Update
      (Transformation|SetRelativeRotation (Variables|Default|GetSM_MonkPilar) (Math|Rotator|MakeRotator (.roll (.rotation _returnvalue)) (.pitch (.rotation _returnvalue)) (+ (.yaw (.rotation _returnvalue)) _rotate)) false false))))

(event EventSelect2
  (bind _sm_monkpilar (Variables|Default|GetSM_MonkPilar))
  (bind _returnvalue (Transformation|GetRelativeTransform _sm_monkpilar))
  (Transformation|SetRelativeRotation (Variables|Default|GetSM_MonkPilar) (Math|Rotator|MakeRotator (.roll (.rotation _returnvalue)) (.pitch (.rotation _returnvalue)) (+ (.yaw (.rotation _returnvalue)) 9e+01)) false false))

(fn ConstructionScript)