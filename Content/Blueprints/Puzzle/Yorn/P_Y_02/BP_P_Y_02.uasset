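; Rotating-pillar puzzle actor (P_Y_02) in which four BP_RotPilar child actors must each face near zero yaw.
; On an uncleared BeginPlay it turns each pillar to a random non-zero quarter turn.
; CheckRotateCorrection shows a light per aligned pillar; all four lit spawns an effect at the energy core and calls MainQuestClear.
; Saved state loads through the game mode, and OnActorLoaded restores lights and marks pillars cleared if solved.
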(event EventBeginPlay
  (CallFunction|InitSetting)
  (if (not (Variables|Default|GetisCleared))
    (CallFunction|InitPuzzleSetting)))

(event EventOnActorLoaded
  (if (Variables|Default|GetisCleared)
    (CallFunction|InitSetting)
    (CallFunction|CheckRotateCorrection)
    (for _array_element (Variables|Default|GetPilars)
      (bind _asbp_rot_pilar (Utilities|Casting|CastToBP_RotPilar (Variables|/Script/Engine.ChildActorComponent|GetChildActor _array_element)))
      (Variables|/Game/Blueprints/Puzzle/Yorn/P_Y_02/BP_RotPilar.BP_RotPilar_C|SetIsCleared _asbp_rot_pilar true))))

(fn ConstructionScript
  (bind _aslutiagame_mode (Utilities|Casting|CastToLUTIAGameMode (Game|GetGameMode)))
  (Class|LUTIAGameMode|LoadActorData _aslutiagame_mode self))

(fn CheckRotateCorrection
  (Utilities|FlowControl|Sequence
    (:then_0
      (bind _return (CallFunction|CheckPilarCompRelativeRotation (Variables|Default|GetBP_RotPilar1)))
      (if _return
        (CallFunction|LightON/OFF 0 false)
        (CallFunction|CheckPuzzleCleared :!label _label)
        (else
          (CallFunction|LightON/OFF 0 true))))
    (:then_1
      (bind _return_2 (CallFunction|CheckPilarCompRelativeRotation (Variables|Default|GetBP_RotPilar2)))
      (if _return_2
        (CallFunction|LightON/OFF 1 false)
        (goto _label)
        (else
          (CallFunction|LightON/OFF 1 true))))
    (:then_2
      (bind _return_3 (CallFunction|CheckPilarCompRelativeRotation (Variables|Default|GetBP_RotPilar3)))
      (if _return_3
        (CallFunction|LightON/OFF 2 false)
        (goto _label)
        (else
          (CallFunction|LightON/OFF 2 true))))
    (:then_3
      (bind _return_4 (CallFunction|CheckPilarCompRelativeRotation (Variables|Default|GetBP_RotPilar4)))
      (if _return_4
        (CallFunction|LightON/OFF 3 false)
        (goto _label)
        (else
          (CallFunction|LightON/OFF 3 true))))))

(fn LightON/OFF
  (params (Index :type Integer) (Hidden :type Boolean))
  (Development|SetHiddeninGame (Utilities|Array|Get(acopy) (Variables|디폴트|GetLights) Index) Hidden false))

(fn CheckPilarCompRelativeRotation
  (params (BP_RotPilar :type Child%20Actor%20Component%20Object%20Reference))
  (bind _asbp_rot_pilar (Utilities|Casting|CastToBP_RotPilar (Variables|/Script/Engine.ChildActorComponent|GetChildActor BP_RotPilar)))
  (return (Math|Float|NearlyEqual(Float) (.yaw (Variables|/Script/Engine.SceneComponent|GetRelativeRotation (Variables|/Game/Blueprints/Puzzle/Yorn/P_Y_02/BP_RotPilar.BP_RotPilar_C|GetSM_MonkPilar _asbp_rot_pilar))) 0.0 1e+01)))

(fn InitSetting
  (Variables|Default|SetPilars (Utilities|Array|MakeArray (Variables|Default|GetBP_RotPilar1) (Variables|Default|GetBP_RotPilar2) (Variables|Default|GetBP_RotPilar3) (Variables|Default|GetBP_RotPilar4)))
  (Variables|디폴트|SetLights (Utilities|Array|MakeArray (Variables|Default|GetLight1) (Variables|Default|GetLight2) (Variables|Default|GetLight3) (Variables|Default|GetLight4))))

(fn InitPuzzleSetting
  (for _array_element (Variables|Default|GetPilars)
    (bind _asbp_rot_pilar (Utilities|Casting|CastToBP_RotPilar (Variables|/Script/Engine.ChildActorComponent|GetChildActor _array_element)))
    (Transformation|SetRelativeRotation (Variables|/Game/Blueprints/Puzzle/Yorn/P_Y_02/BP_RotPilar.BP_RotPilar_C|GetSM_MonkPilar _asbp_rot_pilar) (Math|Rotator|MakeRotator 0.0 0.0 (Math|Conversions|ToFloat(Integer) (* (Math|Random|RandomIntegerinRange 1 3) 90))) false false)))

(fn CheckPuzzleCleared
  (bind _bp_energycore (Variables|Default|GetBP_EnergyCore))
  (bind _returnvalue (Transformation|GetWorldLocation _bp_energycore))
  (for _array_element (Variables|디폴트|GetLights)
    (LocalVariables|SetIsPuzzleClear (and (not (Variables|/Script/Engine.SceneComponent|GetbHiddenInGame _array_element)) (LocalVariables|GetIsPuzzleClear))))
  (if (and (not (Variables|Default|GetisCleared)) (LocalVariables|GetIsPuzzleClear))
    ;[1 1 1] 시네마틱 재생 예정
    (Effects|SpawnEmitteratLocation "/Game/InfinityBladeEffects/Effects/FX_Skill_Leap/P_Skill_Leap_Base_Charge_Weapon.P_Skill_Leap_Base_Charge_Weapon" (Math|Vector|MakeVector (+ (.x _returnvalue) 1e+02) (.y _returnvalue) (.z _returnvalue)) "0, 0, 0" "5.000000,5.000000,5.000000")
    (Variables|Default|SetisCleared true)
    (bind _aslutia_player_state (Utilities|Casting|CastToLUTIA_PlayerState (Game|GetPlayerState 0)))
    (Class|LUTIAPlayerState|MainQuestClear _aslutia_player_state 1)))