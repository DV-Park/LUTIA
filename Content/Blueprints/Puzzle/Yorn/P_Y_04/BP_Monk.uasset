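; Puzzle monk for BP_P_Y_04 that lets the player shift a target monk one fixed step in four directions via dialogue choices.
; GetCommu opens the HUD communication widget and flags the player as communicating.
; Each Select event spawns dust and enables Tick for a single move.
; Tick then has the parent puzzle check transforms, disables itself, clears the communicating flag and removes the dust after a delay.
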(event EventBeginPlay
  (Actor|Tick|SetActorTickEnabled false))

(event EventSelect1
  (Variables|Default|SetUp true)
  (Actor|Tick|SetActorTickEnabled true)
  (bind _returnvalue (Effects|SpawnEmitteratLocation "/Game/InfinityBladeEffects/Effects/FX_Ambient/Fog/P_Dust_Heavy.P_Dust_Heavy" (Transformation|GetWorldLocation (Variables|Default|GetTargetMonk))))
  (Utilities|IsValid (Variables|Default|GetParticle)
    (:Is%20Valid
      (Components|DestroyComponent (Variables|Default|GetParticle)))
    (:Is%20Not%20Valid
      _))
  (Variables|Default|SetParticle _returnvalue))

(event EventSelect3
  (Variables|Default|SetLeft true)
  (Actor|Tick|SetActorTickEnabled true)
  (bind _returnvalue (Effects|SpawnEmitteratLocation "/Game/InfinityBladeEffects/Effects/FX_Ambient/Fog/P_Dust_Heavy.P_Dust_Heavy" (Transformation|GetWorldLocation (Variables|Default|GetTargetMonk))))
  (Utilities|IsValid (Variables|Default|GetParticle)
    (:Is%20Valid
      (Components|DestroyComponent (Variables|Default|GetParticle)))
    (:Is%20Not%20Valid
      _))
  (Variables|Default|SetParticle _returnvalue))

(event EventSelect4
  (Variables|Default|SetRight true)
  (Actor|Tick|SetActorTickEnabled true)
  (bind _returnvalue (Effects|SpawnEmitteratLocation "/Game/InfinityBladeEffects/Effects/FX_Ambient/Fog/P_Dust_Heavy.P_Dust_Heavy" (Transformation|GetWorldLocation (Variables|Default|GetTargetMonk))))
  (Utilities|IsValid (Variables|Default|GetParticle)
    (:Is%20Valid
      (Components|DestroyComponent (Variables|Default|GetParticle)))
    (:Is%20Not%20Valid
      _))
  (Variables|Default|SetParticle _returnvalue))

(event EventGetCommu
  (bind _asbp_third_person_character (Utilities|Casting|CastToBP_ThirdPersonCharacter (Game|GetPlayerCharacter 0)))
  (Variables|Default|SetBP%20Third%20erson%20Chearacter _asbp_third_person_character)
  (bind _aslutiahud (Utilities|Casting|CastToLUTIAHUD (HUD|GetHUD (Game|GetPlayerController 0))))
  (Default|InitCommuc (Variables|/Game/Blueprints/MyBP/LUTIAHUD.LUTIAHUD_C|GetUMG_InGame _aslutiahud) 2)
  (Variables|/Script/LUTIA.LUTIACharacter|SetIsCommunicating (Variables|Default|GetBP%20Third%20erson%20Chearacter) true))

(event EventTick
  (params (DeltaSeconds :type Float%20%28single-precision%29))
  (bind _targetmonk (Variables|Default|GetTargetMonk))
  (if (Math|Boolean|ORBoolean (Variables|Default|GetUp) (Variables|Default|GetDown) (Variables|Default|GetLeft) (Variables|Default|GetRight))
    (if (Variables|Default|GetUp)
      (Variables|Default|SetSign 1)
      (Transformation|AddRelativeLocation _targetmonk "0.000000,-50.000000,0.000000" false false)
      (if true :!label _label
        (Variables|Default|SetUp false)
        (Variables|Default|SetDown false)
        (Variables|Default|SetLeft false)
        (Variables|Default|SetRight false)
        (Utilities|FlowControl|Sequence
          (:then_0
            (bind _asbp_p_y_04 (Utilities|Casting|CastToBP_P_Y_04 (Actor|GetParentActor)))
            (Default|CheckTransformCorrection _asbp_p_y_04))
          (:then_1
            (Actor|Tick|SetActorTickEnabled false)
            (Variables|/Script/LUTIA.LUTIACharacter|SetIsCommunicating (Variables|Default|GetBP%20Third%20erson%20Chearacter) false)
            (Utilities|FlowControl|RetriggerableDelay 5.0)
            (Utilities|IsValid (Variables|Default|GetParticle)
              (:Is%20Valid
                (Components|DestroyComponent (Variables|Default|GetParticle))
                (Variables|Default|SetParticle (Variables|Default|GetParticle)))))))
      (elif (Variables|Default|GetDown)
        (Variables|Default|SetSign -1)
        (Transformation|AddRelativeLocation _targetmonk "0.000000,50.000000,0.000000" false false)
        (goto _label)
        (elif (Variables|Default|GetLeft)
          (Variables|Default|SetSign 0)
          (Transformation|AddRelativeLocation _targetmonk "-50.000000,0.000000,0.000000" false false)
          (goto _label)
          (elif (Variables|Default|GetRight)
            (Variables|Default|SetSign -1)
            (Transformation|AddRelativeLocation _targetmonk "50.000000,0.000000,0.000000" false false)
            (goto _label)))))))

(event EventSelect2
  (Variables|Default|SetDown true)
  (Actor|Tick|SetActorTickEnabled true)
  (bind _returnvalue (Effects|SpawnEmitteratLocation "/Game/InfinityBladeEffects/Effects/FX_Ambient/Fog/P_Dust_Heavy.P_Dust_Heavy" (Transformation|GetWorldLocation (Variables|Default|GetTargetMonk))))
  (Utilities|IsValid (Variables|Default|GetParticle)
    (:Is%20Valid
      (Components|DestroyComponent (Variables|Default|GetParticle)))
    (:Is%20Not%20Valid
      _))
  (Variables|Default|SetParticle _returnvalue))

(fn ConstructionScript)