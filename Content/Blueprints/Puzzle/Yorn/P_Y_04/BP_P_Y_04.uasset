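; Monk-alignment puzzle actor (P_Y_04) that completes main quest step 3 when all four monks are centred.
; On BeginPlay it hides four torch fires and randomly offsets each child monk's TargetMonk in X/Y.
; CheckTransformCorrection, not called within this graph, lights each monk's fire when its relative position nears zero.
; With all fires visible, it spawns an AOE emitter, raises the altar and notifies LUTIA_PlayerState.
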(event EventBeginPlay
  (CallFunction|InitSetting)
  (CallFunction|InitPuzzleSetting))

(fn ConstructionScript)

(fn InitSetting
  (Variables|Default|SetMonk (Utilities|Array|MakeArray (Variables|Default|GetBP_Monk1) (Variables|Default|GetBP_Monk2) (Variables|Default|GetBP_Monk3) (Variables|Default|GetBP_Monk4)))
  (bind _output_get (Variables|Default|SetFire (Utilities|Array|MakeArray (Variables|Default|GetP_TorchFire_Entrance1) (Variables|Default|GetP_TorchFire_Entrance2) (Variables|Default|GetP_TorchFire_Entrance3) (Variables|Default|GetP_TorchFire_Entrance4))))
  (for _array_element _output_get
    (Development|SetHiddeninGame _array_element true false)))

(fn InitPuzzleSetting
  (bind _returnvalue (Math|Random|RandomIntegerinRange -2 -1))
  (bind _returnvalue_2 (* _returnvalue 50))
  (for _array_element (Variables|Default|GetMonk)
    (bind _asbp_monk (Utilities|Casting|CastToBP_Monk (Variables|/Script/Engine.ChildActorComponent|GetChildActor _array_element)))
    (Transformation|AddRelativeLocation (Variables|/Game/Blueprints/Puzzle/Yorn/P_Y_04/BP_Monk.BP_Monk_C|GetTargetMonk _asbp_monk) (Math|Vector|MakeVector (Math|Conversions|ToFloat(Integer) _returnvalue_2) (Math|Conversions|ToFloat(Integer) _returnvalue_2) 0.0) false false)))

(fn CheckTransformCorrection
  (Utilities|FlowControl|Sequence
    (:then_0
      (bind _return (CallFunction|CheckMonkCompRelativePosition (Variables|Default|GetBP_Monk1)))
      (if _return
        (CallFunction|EffectON/OFF 0 false)
        (CallFunction|CheckPuzzleCleared :!label _label)
        (else
          (CallFunction|EffectON/OFF 0 true))))
    (:then_1
      (bind _return_2 (CallFunction|CheckMonkCompRelativePosition (Variables|Default|GetBP_Monk2)))
      (if _return_2
        (CallFunction|EffectON/OFF 1 false)
        (goto _label)
        (else
          (CallFunction|EffectON/OFF 1 true))))
    (:then_2
      (bind _return_3 (CallFunction|CheckMonkCompRelativePosition (Variables|Default|GetBP_Monk3)))
      (if _return_3
        (CallFunction|EffectON/OFF 2 false)
        (goto _label)
        (else
          (CallFunction|EffectON/OFF 2 true))))
    (:then_3
      (bind _return_4 (CallFunction|CheckMonkCompRelativePosition (Variables|Default|GetBP_Monk4)))
      (if _return_4
        (CallFunction|EffectON/OFF 3 false)
        (goto _label)
        (else
          (CallFunction|EffectON/OFF 3 true))))))

(fn CheckMonkCompRelativePosition
  (params (BP_Monk :type Child%20Actor%20Component%20Object%20Reference))
  (bind _asbp_monk (Utilities|Casting|CastToBP_Monk (Variables|/Script/Engine.ChildActorComponent|GetChildActor BP_Monk)))
  (return (and (Math|Float|NearlyEqual(Float) (.x (Variables|/Script/Engine.SceneComponent|GetRelativeLocation (Variables|/Game/Blueprints/Puzzle/Yorn/P_Y_04/BP_Monk.BP_Monk_C|GetTargetMonk _asbp_monk))) 0.0 1e+01) (Math|Float|NearlyEqual(Float) (.y (Variables|/Script/Engine.SceneComponent|GetRelativeLocation (Variables|/Game/Blueprints/Puzzle/Yorn/P_Y_04/BP_Monk.BP_Monk_C|GetTargetMonk _asbp_monk))) 0.0 1e+01))))

(fn EffectON/OFF
  (params (Index :type Integer) (Hidden :type Boolean))
  (Development|SetHiddeninGame (Utilities|Array|Get(acopy) (Variables|Default|GetFire) Index) Hidden false))

(fn CheckPuzzleCleared
  (for _array_element (Variables|Default|GetFire)
    (LocalVariables|SetIsPuzzleClear (and (not (Variables|/Script/Engine.SceneComponent|GetbHiddenInGame _array_element)) (LocalVariables|GetIsPuzzleClear))))
  (if (LocalVariables|GetIsPuzzleClear)
    (Effects|SpawnEmitteratLocation "/Game/InfinityBladeEffects/Effects/FX_Monsters/FX_Monster_Ausar/P_AU_ShieldSlam_AOE.P_AU_ShieldSlam_AOE" (Math|Vector|MakeVector 0.0 0.0 0.0) "0, 0, 0" "5.000000,5.000000,5.000000")
    (if (LocalVariables|GetIsPuzzleClear)
      (Transformation|AddRelativeLocation (Variables|Default|GetSM_AltarBase) "0.000000,0.000000,100.000000" false false)
      (bind _aslutia_player_state (Utilities|Casting|CastToLUTIA_PlayerState (Game|GetPlayerState 0)))
      (Class|LUTIAPlayerState|MainQuestClear _aslutia_player_state 3))))