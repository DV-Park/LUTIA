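; Puzzle trigger box that detects when two different Wolf actors have entered it.
; Box overlaps add new wolves to OverlappedWolf and raise Count, which never drops on exit.
; At two, it plays an aura effect after a delay, increments the parent BP_ClearBox's Count, then calls ClearPuzzle after another delay.
; Flag blocks repeat wolves but is never reset, so one repeat overlap stops all further counting.
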(event OnComponentBeginOverlap(Box)
  (params (OverlappedComponent :type Primitive%20Component%20Object%20Reference) (OtherActor :type Actor%20Object%20Reference) (OtherComp :type Primitive%20Component%20Object%20Reference) (OtherBodyIndex :type Integer) (bFromSweep :type Boolean) (SweepResult :type Hit%20Result%20Structure%20%28by%20ref%29))
  (for _array_element (Variables|Default|GetOverlappedWolf)
    (if (== OtherActor _array_element)
      (Variables|Default|SetFlag true)))
  (if (not (Variables|Default|GetFlag))
    (bind _aswolf (Utilities|Casting|CastToWolf OtherActor))
    (Math|Integer|IncrementInt (Variables|Default|GetCount)
      (:%20%20
        (Development|PrintString "Hello")
        (Utilities|Array|Add (Variables|Default|GetOverlappedWolf) _aswolf)
        (if (== (Variables|Default|GetCount) 2)
          (Utilities|FlowControl|Delay 1.0)
          (Effects|SpawnEmitteratLocation "/Game/InfinityBladeEffects/Effects/FX_Skill_Aura/P_Aura_Default_Upheaval_01.P_Aura_Default_Upheaval_01" (Transformation|GetWorldLocation (Variables|Default|GetBox)) "0, 0, 0" "3.000000,3.000000,3.000000")
          (bind _asbp_clear_box (Utilities|Casting|CastToBP_ClearBox (Actor|GetParentActor)))
          (Math|Integer|IncrementInt (Variables|/Game/Blueprints/Puzzle/Yorn/P_Y_03/BP_ClearBox.BP_ClearBox_C|GetCount _asbp_clear_box)
            (:%20%20
              (Utilities|FlowControl|Delay 2.0)
              (Default|ClearPuzzle _asbp_clear_box)))
          (else
            (Development|PrintString "1")))))))

(fn ConstructionScript)