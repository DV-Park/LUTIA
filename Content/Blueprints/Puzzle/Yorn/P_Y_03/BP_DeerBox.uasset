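; BP_DeerBox is a puzzle trigger volume that tracks deer entering its box.
; On overlap it ignores actors already in its OverlappedDeer list, then counts and records each new Deer1.
; When the fourth deer is counted it spawns a shield-slam emitter at a hardcoded world location; other counts are only printed to screen.
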(event OnComponentBeginOverlap(Box)
  (params (OverlappedComponent :type Primitive%20Component%20Object%20Reference) (OtherActor :type Actor%20Object%20Reference) (OtherComp :type Primitive%20Component%20Object%20Reference) (OtherBodyIndex :type Integer) (bFromSweep :type Boolean) (SweepResult :type Hit%20Result%20Structure%20%28by%20ref%29))
  (bind _count (Variables|Default|GetCount))
  (for _array_element (Variables|Default|GetOverlappedDeer)
    (if (== OtherActor _array_element)
      (Variables|Default|SetFlag true)))
  (if (not (Variables|Default|GetFlag))
    (bind _asdeer_1 (Utilities|Casting|CastToDeer1 OtherActor))
    (Math|Integer|IncrementInt (Variables|Default|GetCount)
      (:%20%20
        (Utilities|Array|Add (Variables|Default|GetOverlappedDeer) _asdeer_1)
        (if (== _count 4)
          (Effects|SpawnEmitteratLocation "/Game/InfinityBladeEffects/Effects/FX_Monsters/FX_Monster_Ausar/P_AU_ShieldSlam_AOE.P_AU_ShieldSlam_AOE" "-185462.047595,-134220.168784,-13409.335834" "0, 0, 0" "3.000000,3.000000,3.000000")
          (else
            (Development|PrintString (Utilities|String|ToString(Integer) _count))))))))

(fn ConstructionScript)