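; BP_Random is a puzzle floor pad that toggles itself and its adjacent pads when stepped on, in the style of Lights Out.
; A box overlap by BP_ThirdPersonCharacter flips IsOn on the pad and on each entry in AdjacentPads.
; This pad's Count tracks only the neighbor flips and prints after each one; no solved check exists here.
; Tick sets the base support material from IsOn every frame.
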(event OnComponentBeginOverlap(Box)
  (params (OverlappedComponent :type Primitive%20Component%20Object%20Reference) (OtherActor :type Actor%20Object%20Reference) (OtherComp :type Primitive%20Component%20Object%20Reference) (OtherBodyIndex :type Integer) (bFromSweep :type Boolean) (SweepResult :type Hit%20Result%20Structure%20%28by%20ref%29))
  (if (== (Utilities|GetClass OtherActor) "/Game/ThirdPerson/Blueprints/BP_ThirdPersonCharacter.BP_ThirdPersonCharacter_C")
    (if (Variables|Default|GetisOn)
      (Variables|Default|SetisOn false)
      (else
        (Variables|Default|SetisOn true)))
    (for _array_element (Variables|Default|GetAdjacentPads)
      (if (Variables|BP_Random_C|GetisOn _array_element)
        (Variables|BP_Random_C|SetisOn _array_element false)
        (Math|Integer|DecrementInt (Variables|Default|Getcount)
          (:%20%20
            _))
        (else
          (Variables|BP_Random_C|SetisOn _array_element true)
          (Math|Integer|IncrementInt (Variables|Default|Getcount)
            (:%20%20
              _))))
      (Development|PrintString (Utilities|String|ToString(Integer) (Variables|Default|Getcount))))))

(event EventTick
  (params (DeltaSeconds :type Float%20%28single-precision%29))
  (bind _sm_basesupport (Variables|Default|GetSM_BaseSupport))
  (if (Variables|Default|GetisOn)
    (Rendering|Material|SetMaterial _sm_basesupport 0 "/Game/GothicTemple/Environment/Props/OldTemple/OldTemple/MI_OldTemple_03.MI_OldTemple_03")
    (else
      (Rendering|Material|SetMaterial _sm_basesupport 0 "/Game/Blueprints/Puzzle/Yorn/P_Y_01/isOff_Inst50.isOff_Inst50"))))

(fn ConstructionScript)