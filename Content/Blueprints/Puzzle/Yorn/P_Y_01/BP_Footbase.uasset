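; Footplate puzzle that manages nine BP_Random child actors as pads, where stepping on one changes the state of linked pads.
; When BP_Gavin overlaps a pad, the flagged pad's ComPad indices select which pads get SetBaseState, then every pad's IsOn is checked.
; Solving it fires a Niagara-style missile effect, clears main quest 0, plays a cinematic and deactivates pad missiles.
; LUTIAGameMode loads saved data, and OnActorLoaded reapplies pad states if cleared.
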(event Custom|커스텀이벤트
  (params (OverlappedComponent :type Primitive%20Component%20Object%20Reference) (OtherActor :type Actor%20Object%20Reference) (OtherComp :type Primitive%20Component%20Object%20Reference) (OtherBodyIndex :type Integer) (bFromSweep :type Boolean) (SweepResult :type Hit%20Result%20Structure%20%28by%20ref%29))
  (if (== (Utilities|GetClass OtherActor) "/Game/MetaHumans/GavinBP/BP_Gavin.BP_Gavin_C")
    (CallFunction|ChangeOtherFootBase)
    (CallFunction|CheckPuzzleClear)))

(event EventBeginPlay
  (for _array_element (Variables|Default|GetFootBase)
    (bind _asbp_random (Utilities|Casting|CastToBP_Random (Variables|/Script/Engine.ChildActorComponent|GetChildActor _array_element)))
    (Collision|BindEventtoOnComponentBeginOverlap (Variables|/Game/Blueprints/Puzzle/Yorn/P_Y_01/BP_Random.BP_Random_C|GetBox _asbp_random) (delegate Custom|커스텀이벤트))))

(event EventOnActorLoaded
  (if (Variables|Default|GetisCleared)
    (for _array_element (Variables|Default|GetFootBase)
      (bind _asbp_random (Utilities|Casting|CastToBP_Random (Variables|/Script/Engine.ChildActorComponent|GetChildActor _array_element)))
      (Default|SetBaseState _asbp_random))))

(fn ConstructionScript
  (Variables|Default|SetFootBase (Utilities|Array|MakeArray (Variables|Default|GetBase1) (Variables|Default|GetBase2) (Variables|Default|GetBase3) (Variables|Default|GetBase4) (Variables|Default|GetBase5) (Variables|Default|GetBase6) (Variables|Default|GetBase7) (Variables|Default|GetBase8) (Variables|Default|GetBase9)))
  (bind _aslutiagame_mode (Utilities|Casting|CastToLUTIAGameMode (Game|GetGameMode)))
  (Class|LUTIAGameMode|LoadActorData _aslutiagame_mode self))

(fn CheckPuzzleClear
  (for _array_element (Variables|Default|GetFootBase)
    (bind _asbp_random (Utilities|Casting|CastToBP_Random (Variables|/Script/Engine.ChildActorComponent|GetChildActor _array_element)))
    (LocalVariables|SetisPuzzleClear (and (LocalVariables|GetisPuzzleClear) (Variables|/Game/Blueprints/Puzzle/Yorn/P_Y_01/BP_Random.BP_Random_C|GetisOn _asbp_random))))
  (if (LocalVariables|GetisPuzzleClear)
    (Variables|Default|SetisCleared true)
    (CallFunction|VFXon)
    (bind _aslutia_player_state (Utilities|Casting|CastToLUTIA_PlayerState (Game|GetPlayerState 0)))
    (Class|LUTIAPlayerState|MainQuestClear _aslutia_player_state)
    (Default|CallCallCinematic)
    (for _array_element_2 (Variables|Default|GetFootBase)
      (bind _asbp_random_2 (Utilities|Casting|CastToBP_Random (Variables|/Script/Engine.ChildActorComponent|GetChildActor _array_element_2)))
      (Components|Activation|Deactivate (Variables|/Game/Blueprints/Puzzle/Yorn/P_Y_01/BP_Random.BP_Random_C|GetMissiles _asbp_random_2)))))

(fn ChangeOtherFootBase
  (for _array_element (Variables|Default|GetFootBase)
    (bind _asbp_random (Utilities|Casting|CastToBP_Random (Variables|/Script/Engine.ChildActorComponent|GetChildActor _array_element)))
    (if (Variables|/Game/Blueprints/Puzzle/Yorn/P_Y_01/BP_Random.BP_Random_C|GetFlag _asbp_random)
      (LocalVariables|SetSetBase (Variables|/Game/Blueprints/Puzzle/Yorn/P_Y_01/BP_Random.BP_Random_C|GetComPad _asbp_random))
      (Variables|/Game/Blueprints/Puzzle/Yorn/P_Y_01/BP_Random.BP_Random_C|SetFlag _asbp_random false)))
  (for _array_element_2 (LocalVariables|GetSetBase)
    (bind _asbp_random_2 (Utilities|Casting|CastToBP_Random (Variables|/Script/Engine.ChildActorComponent|GetChildActor (Utilities|Array|Get(acopy) (Variables|Default|GetFootBase) (- _array_element_2 1)))))
    (Default|SetBaseState _asbp_random)))

(fn VFXon
  (Components|Activation|Activate (Variables|Default|GetMissile) false)
  (Niagara|SetNiagaraVariable(Vector3) (Variables|Default|GetMissile) "Target" "-210614.000000,-154329.000000,-12312.000000")
  (Utilities|Time|SetTimerbyEvent (EventDispatchers|CreateEvent :!event Test) 2.0))

(fn Test
  (Components|Activation|Deactivate (Variables|Default|GetMissile)))